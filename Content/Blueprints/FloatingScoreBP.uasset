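; Floating score actor that shows a score widget in the world, then fades it out and removes itself.
; On BeginPlay, it turns the Score widget component once toward the player camera.
; After a short delay it calls FadeOutScore on the WB_FloatingScore widget, waits for the fade, then destroys the actor.
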(event `self.ReceiveBeginPlay`
  ;[1 1 1] After spawning text, delay then fade out before destroying itself.
  (`SceneComponent.K2_SetWorldRotation` (`self.Score`) (`KismetMathLibrary.FindLookAtRotation` (`SceneComponent.K2_GetComponentLocation` (`self.Score`)) (`PlayerCameraManager.GetCameraLocation` (`GameplayStatics.GetPlayerCameraManager` 0))) false false)
  (`KismetSystemLibrary.Delay` 0.2)
  (bind _aswb_floating_score (cast `/Game/UI/WB_FloatingScore` (`WidgetComponent.GetUserWidgetObject` (`self.Score`))))
  (`/Game/UI/WB_FloatingScore.FadeOutScore` _aswb_floating_score)
  (`KismetSystemLibrary.Delay` 1.0)
  (`self.K2_DestroyActor`))

(fn `UserConstructionScript`)